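; Player controller that drives a visual-novel style prologue, adding the input mapping context and creating the background and main text widgets.
; The main input either completes the line being typed or loads the next DT_Prolog row by counter, setting text and background and appending to a history string.
; A Delay on Tick paces a typewriter effect that moves characters from the pending string into the displayed text.
; The history input prints the accumulated text as debug output.
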(event `self.ReceiveBeginPlay`
  (`EnhancedInputSubsystemInterface.AddMappingContext` (subsystem `EnhancedInputLocalPlayerSubsystem`) "/Game/Input/IMC/IMC_Main.IMC_Main" 0 (struct))
  (bind _returnvalue (`|CreateWidget` "/Game/UI/UI_BG.UI_BG_C"))
  (bind _output_get (set `self.UI_BG` _returnvalue))
  (`UserWidget.AddToViewport` _output_get 0)
  (bind _returnvalue_2 (`|CreateWidget` "/Game/UI/UI_MainText.UI_MainText_C"))
  (bind _output_get_2 (set `self.MainTextUI` _returnvalue_2))
  (`UserWidget.AddToViewport` _output_get_2 0))

(event `EnhancedInput|/Game/Input/IA_Main`
  (params (ActionValue :type Boolean) (ElapsedSeconds :type "Float (double-precision)") (TriggeredSeconds :type "Float (double-precision)") (InputAction :type "InputAction Object Reference" :default "/Game/Input/IA_Main.IA_Main"))
  (bind _returnvalue (`KismetStringLibrary.Conv_StringToName` (`KismetStringLibrary.Conv_IntToString` (`self.TextCount`))))
  (:`Started`
    (if (>= (`KismetStringLibrary.Len` (`self.NewText`)) 1)
      (set `self.Text` (`self.NewText2`))
      (set `self.NewText` "")
      (set `self.NewText2` "")
      (else
        (set `self.Text` "")
        (bind _returnvalue_2 (`|GetDataTableRow` "/Game/DataTable/DT_Prolog.DT_Prolog" _returnvalue)
          (:`then`
            (bind _text (break `/Game/Structure/ST_MainText` _returnvalue_2))
            (set `self.NewText` _text)
            (set `self.NewText2` _text)
            (set `self.AllText` (`KismetStringLibrary.Concat_StrStr` (`self.AllText`) " \n" _text))
            (bind _returnvalue_3 (`|GetDataTableRow` "/Game/DataTable/DT_Prolog.DT_Prolog" _returnvalue)
              (:`then`
                (set `self.BG` (`.BG_8_ACBBB8E14D425FF04D2A82BA9BDC8C12` (break `/Game/Structure/ST_MainText` _returnvalue_3)))
                (bind _result (`/Engine/EditorBlueprintResources/StandardMacros.IncrementInt` (`self.TextCount`))
                  (:`  `
                    (set `self.TextCount` _result)))))))))))

(event `self.ReceiveTick`
  (params (DeltaSeconds :type "Float (single-precision)"))
  (bind _newtext (`self.NewText`))
  (`KismetSystemLibrary.Delay` 0.05)
  (set `self.Text` (`KismetStringLibrary.Concat_StrStr` (`self.Text`) (`KismetStringLibrary.Left` _newtext (`self.AddTextCount`))))
  (set `self.NewText` (`KismetStringLibrary.RightChop` _newtext 1)))

(event `EnhancedInput|/Game/Input/IA_History`
  (params (ActionValue :type Boolean) (ElapsedSeconds :type "Float (double-precision)") (TriggeredSeconds :type "Float (double-precision)") (InputAction :type "InputAction Object Reference" :default "/Game/Input/IA_History.IA_History"))
  (:`Started`
    (`KismetSystemLibrary.PrintString` (`self.AllText`))))

(fn `UserConstructionScript`)